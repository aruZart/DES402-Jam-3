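; Dining room dialogue component that scripts a branching family conversation in which relatives press the player about having kids.
; The Dialogue override calls its parent, then chains AddDialogue nodes, branching on option index and rejoining at shared lines.
; Only the health concerns answer to the final question sets IsDiningRoomFinished, switches to tree index 1 and closes the conversation; the other two repeat the question.
; DiningRoomDialogue is an empty stub.
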(event EventBeginPlay)

(event EventTick
  (params (DeltaSeconds :type Float%20%28single-precision%29)))

(fn DiningRoomDialogue)

(fn Dialogue
  (|CallParentFunction)
  (bind (_state _option_index) (CallFunction|AddDialogue "Uncle" "Hey kiddo, how has life been?" (Utilities|Array|MakeArray "I'm a grown adult, don't call me 'kiddo'" "You live in the same world I do, terrible.")))
  (switch Utilities|FlowControl|Switch|SwitchonEnum_DialogueState _state
    (:NewEnumerator0
      (switch int _option_index
        (:0
          (bind _state_2 (CallFunction|AddDialogue "Uncle" "That's right, all grown up now, huh?" (Utilities|Array|MakeArray "Continue")))
          (switch Utilities|FlowControl|Switch|SwitchonEnum_DialogueState _state_2
            (:NewEnumerator0
              (bind _state_3 (CallFunction|AddDialogue "Mum" "*Mum turns to him for a second with judgemental eyes, you aren't 'grown up' to her*" (Utilities|Array|MakeArray "Continue")))
              (switch Utilities|FlowControl|Switch|SwitchonEnum_DialogueState _state_3
                (:NewEnumerator0
                  (bind _state_4 (CallFunction|AddDialogue "Uncle" "U-Uh... right, of course, so... " (Utilities|Array|MakeArray "Continue")))
                  (switch Utilities|FlowControl|Switch|SwitchonEnum_DialogueState _state_4
                    (:NewEnumerator0
                      _)))))))
        (:1
          (bind _state_5 (CallFunction|AddDialogue "Aunt" "Oh please! It's not that bad!" (Utilities|Array|MakeArray "Continue")))
          (switch Utilities|FlowControl|Switch|SwitchonEnum_DialogueState _state_5
            (:NewEnumerator0
              (bind _state_6 (CallFunction|AddDialogue "Dad" "I don't know, I think things feel a bit \"up-in-the-air\" at the moment..." (Utilities|Array|MakeArray "Continue")))
              (switch Utilities|FlowControl|Switch|SwitchonEnum_DialogueState _state_6
                (:NewEnumerator0
                  (bind _state_7 (CallFunction|AddDialogue "Uncle" "Let's not talk about that stuff here..." (Utilities|Array|MakeArray "Continue")))
                  (switch Utilities|FlowControl|Switch|SwitchonEnum_DialogueState _state_7
                    (:NewEnumerator0
                      _))))))))
      (bind _state_8 (CallFunction|AddDialogue "Uncle" "Let's talk on the brighter side, hey? " (Utilities|Array|MakeArray "Continue")))
      (switch Utilities|FlowControl|Switch|SwitchonEnum_DialogueState _state_8
        (:NewEnumerator0
          (bind _state_9 (CallFunction|AddDialogue "Uncle" "So... when are you having kids?" (Utilities|Array|MakeArray "Continue")))
          (switch Utilities|FlowControl|Switch|SwitchonEnum_DialogueState _state_9
            (:NewEnumerator0
              (bind (_state_10 _option_index_2) (CallFunction|AddDialogue "Mum" "When are you gonna bless your parents with a grand child?" (Utilities|Array|MakeArray "I'm not exactly planning on it..." "Fuck off. I'm not having kids.")))
              (switch Utilities|FlowControl|Switch|SwitchonEnum_DialogueState _state_10
                (:NewEnumerator0
                  (switch int _option_index_2
                    (:0
                      (bind _state_11 (CallFunction|AddDialogue "Dad" "Is that going to change eventually?" (Utilities|Array|MakeArray "I shouldn't need to explain myself.")))
                      (switch Utilities|FlowControl|Switch|SwitchonEnum_DialogueState _state_11
                        (:NewEnumerator0
                          _)))
                    (:1
                      (bind _state_12 (CallFunction|AddDialogue "Mum" "See? So childish!" (Utilities|Array|MakeArray "Continue")))
                      (switch Utilities|FlowControl|Switch|SwitchonEnum_DialogueState _state_12
                        (:NewEnumerator0
                          (bind _state_13 (CallFunction|AddDialogue "Uncle" "Hey now, no need for aggression..." (Utilities|Array|MakeArray "Continue")))
                          (switch Utilities|FlowControl|Switch|SwitchonEnum_DialogueState _state_13
                            (:NewEnumerator0
                              _))))))
                  (bind (_state_14 _option_index_3) (CallFunction|AddDialogue "Uncle" "Why don't you want kids?" (Utilities|Array|MakeArray "Have you thought of the health concerns?" "Do you have any clue how much that would cost?" "What about the world we live in?") :!label _label))
                  (switch Utilities|FlowControl|Switch|SwitchonEnum_DialogueState _state_14
                    (:NewEnumerator0
                      (switch int _option_index_3
                        (:0
                          (Variables|Default|SetisDiningRoomFinished true)
                          (CallFunction|SetDialogueTreeIndex 1)
                          (CallFunction|CloseConversation))
                        (:1
                          (switch Utilities|FlowControl|Switch|SwitchonEnum_DialogueState _state_14 :!label _label_2
                            (:NewEnumerator0
                              (goto _label))))
                        (:2
                          (goto _label_2))))))))))))))