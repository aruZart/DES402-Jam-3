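; BP_Interact_Base is a base interactable Blueprint with text components for an item name and an interaction prompt.
; The construction script fills the name text from ItemName.
; SetInteractableState shows or hides both texts based on whether interaction can be shown.
; ConversationClosed relays a ConversationClosedMessage to the InteractInstigator.
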(event EventSetInteractableState
  (params (bCanShowInteract? :type Boolean))
  (bind _txt_itemname (Variables|Default|GetTxt_ItemName))
  (bind _txt_textprompt (Variables|Default|GetTxt_TextPrompt))
  (if bCanShowInteract?
    (Rendering|SetVisibility _txt_itemname true false)
    (Rendering|SetVisibility _txt_textprompt true false)
    (else
      (Rendering|SetVisibility _txt_itemname false false)
      (Rendering|SetVisibility _txt_textprompt false false))))

(event EventConversationClosed
  (Class|BPIInteractable|ConversationClosed(Message) (Variables|Default|GetInteractInstigator)))

(fn ConstructionScript
  (Rendering|Components|TextRender|SetText (Variables|Default|GetTxt_ItemName) (Variables|Default|GetItemName)))