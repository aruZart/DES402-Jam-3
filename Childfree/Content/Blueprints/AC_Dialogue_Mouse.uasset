(fn Dialogue
  (|CallParentFunction)
  (switch int (Variables|Default|GetDialogueTreeIndex)
    (:0
      (bind (_state _option_index) (CallFunction|AddDialogue "Mouse" "Hi, do you have any cheese?" (Utilities|Array|MakeArray "Yes" "No")))
      (switch Utilities|FlowControl|Switch|SwitchonEnum_DialogueState _state
        (:NewEnumerator0
          (switch int _option_index
            (:0
              (bind (_state_2 _option_index_2) (CallFunction|AddDialogue "Mouse" "Ahh, that's great news! Can I get a slice mayhaps?" (Utilities|Array|MakeArray "Give Cheese" "Keep Cheese")))
              (switch Utilities|FlowControl|Switch|SwitchonEnum_DialogueState _state_2
                (:NewEnumerator0
                  (switch int _option_index_2
                    (:0
                      (bind _state_3 (CallFunction|AddDialogue "Mouse" "Thank you for the fine slice!" (Utilities|Array|MakeArray "Continue")))
                      (switch Utilities|FlowControl|Switch|SwitchonEnum_DialogueState _state_3
                        (:NewEnumerator0
                          (CallFunction|SetDialogueTreeIndex 1)
                          (CallFunction|CloseConversation))))
                    (:1
                      ;[0.15 0.15 0.15 0.5] Goes back to previous dialogue prompt
                      (bind _state_4 (CallFunction|AddDialogue "Mouse" "Greedy bugger!" (Utilities|Array|MakeArray "Continue")))
                      (switch Utilities|FlowControl|Switch|SwitchonEnum_DialogueState _state_4
                        (:NewEnumerator0
                          ;;[0.15 0 0 0.5] Progress steps = amount of prompts back
                          (CallFunction|RemoveDialogueProgress 2)
                          (CallFunction|CloseConversation))))))))
            (:1
              ;[0.15 0.15 0.15 0.5] Resets back to start of dialogue tree prompt
              (bind _state_5 (CallFunction|AddDialogue "Mouse" "Dang..." (Utilities|Array|MakeArray "Continue")))
              (switch Utilities|FlowControl|Switch|SwitchonEnum_DialogueState _state_5
                (:NewEnumerator0
                  (CallFunction|ClearDialogueProgress)
                  (CallFunction|CloseConversation))))))))
    (:1
      ;[0.15 0.15 0.15 0.5] Prompt appears when certain prompts were triggered i.e. you've given the cheese to the mouse
      (bind _state_6 (CallFunction|AddDialogue "Mouse" (Utilities|Select :Index (Math|Random|RandomIntegerinRange 0 1) :Option%200 "Mmmmmm!" :Option%201 "You're such a nice bloke! Thanks again! :3") (Utilities|Array|MakeArray "Continue")))
      (switch Utilities|FlowControl|Switch|SwitchonEnum_DialogueState _state_6
        (:NewEnumerator0
          (CallFunction|ClearDialogueProgress)
          (CallFunction|CloseConversation))))))